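; BP_Player drives a looping showcase of a player attack animation with timeline-animated base and staff lights, restarting after a delay.
; SpawnDragon spawns temporary dragon and emitter skeletal meshes at the player's BuildUpSocket, minus an offset, moved by timelines.
; Niagara detail and trail systems attach to them, while timelines animate dissolve, eyes and mouth on a shared dynamic dragon material.
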(event Custom|SpawnDragon
  ;[0.1779 0.000303 0.0319] DragonSpawn
  (Utilities|FlowControl|Sequence
    (:then_0
      (bind _returnvalue (Game|SpawnActorfromClass "/Script/Engine.SkeletalMeshActor" (Math|Transform|MakeTransform (- (.location (Transformation|GetSocketTransform (Variables|Default|GetPlayer) "BuildUpSocket" "RTS_World")) (Variables|Default|GetDragonOffset)) "0, 0, 0" "1.000000,1.000000,1.000000") "Undefined" "MultiplyWithRoot" 0 0))
      (Rendering|Material|SetMaterial (Variables|/Script/Engine.SkeletalMeshActor|GetSkeletalMeshComponent _returnvalue) 0 (stale EventBeginPlay _output_get))
      (Utilities|FlowControl|Sequence
        (:then_0
          (Components|SkeletalMesh|SetSkeletalMeshAsset (Variables|/Script/Engine.SkeletalMeshActor|GetSkeletalMeshComponent _returnvalue) "/Game/Abschlussarbeit/Meshes/SKM_Dragon.SKM_Dragon")
          (Components|Animation|PlayAnimation (Variables|/Script/Engine.SkeletalMeshActor|GetSkeletalMeshComponent _returnvalue) "/Game/Abschlussarbeit/Animations/Anim_Dragon.Anim_Dragon" true)
          (bind _output_get (Variables|Default|SetStartPosition (Transformation|GetActorLocation _returnvalue)))
          (bind _move (Timeline|DragonMovement PlayFromStart)
            (:Update
              (Transformation|SetActorLocation _returnvalue (+ _move _output_get) false false))
            (:Finished
              (Utilities|FlowControl|Delay 0.5)
              (Actor|DestroyActor _returnvalue))))
        (:then_1
          (bind _returnvalue_2 (AddComponent|AddSceneComponent _returnvalue false))
          (Niagara|SpawnSystemAttached "/Game/Abschlussarbeit/NiagaraSystems/NS_DragonDetails.NS_DragonDetails" _returnvalue_2 "None" "0, 0, 0" "0, 0, 0" "KeepRelativeOffset" false))
        (:then_2
          (bind _newtrack_0 (Timeline|DragonMaterial PlayFromStart)
            (:Update
              (Rendering|Material|SetScalarParameterValue (Variables|Default|GetDragonMAT) "Dissolve[1-0]" _newtrack_0 :!class /Script/Engine.MaterialInstanceDynamic))))
        (:then_3
          (bind _eyes (Timeline|DragonEyes PlayFromStart)
            (:Update
              (Rendering|Material|SetScalarParameterValue (Variables|Default|GetDragonMAT) "Eyes" _eyes :!class /Script/Engine.MaterialInstanceDynamic))))
        (:then_4
          (bind _mouth (Timeline|Mouth Play)
            (:Update
              (Rendering|Material|SetScalarParameterValue (Variables|Default|GetDragonMAT) "Mouth" _mouth :!class /Script/Engine.MaterialInstanceDynamic))))))
    (:then_1
      (bind _returnvalue_3 (Game|SpawnActorfromClass "/Script/Engine.SkeletalMeshActor" (Math|Transform|MakeTransform (- (.location (Transformation|GetSocketTransform (Variables|Default|GetPlayer) "BuildUpSocket" "RTS_World")) (Variables|Default|GetDragonOffset)) "0, 0, 0" "1.000000,1.000000,1.000000") "Undefined" "MultiplyWithRoot" 0 0))
      (Utilities|FlowControl|Sequence
        (:then_0
          (Components|SkeletalMesh|SetSkeletalMeshAsset (Variables|/Script/Engine.SkeletalMeshActor|GetSkeletalMeshComponent _returnvalue_3) "/Game/Abschlussarbeit/Meshes/SKM_EmitterMesh.SKM_EmitterMesh")
          (Components|Animation|PlayAnimation (Variables|/Script/Engine.SkeletalMeshActor|GetSkeletalMeshComponent _returnvalue_3) "/Game/Abschlussarbeit/Animations/Anim_Emitter.Anim_Emitter" true)
          (bind _output_get_2 (Variables|Default|SetStartPosition (Transformation|GetActorLocation _returnvalue_3)))
          (bind _move_2 (Timeline|Timeline_2 Play)
            (:Update
              (Transformation|SetActorLocation _returnvalue_3 (+ _move_2 _output_get_2) false false))
            (:Finished
              (Utilities|FlowControl|Delay 0.2)
              (Actor|DestroyActor _returnvalue_3))))
        (:then_1
          (bind _returnvalue_4 (AddComponent|AddSceneComponent _returnvalue_3 false))
          (Utilities|FlowControl|Delay 0.15)
          (Niagara|SpawnSystemAttached "/Game/Abschlussarbeit/NiagaraSystems/NS_DragonTrails.NS_DragonTrails" _returnvalue_4 "None" "0, 0, 0" "0, 0, 0" "KeepRelativeOffset" false))))))

(event EventBeginPlay
  ;[1 0.6308 0.2789] Lights
  (bind _returnvalue (Rendering|Material|CreateDynamicMaterialInstance "/Game/Abschlussarbeit/Materials/M_Dragon.M_Dragon" "None" "None" :!class /Script/Engine.KismetMaterialLibrary))
  (bind _output_get (Variables|Default|SetDragonMAT _returnvalue))
  (Components|Animation|PlayAnimation (Variables|Default|GetPlayer) "/Game/Abschlussarbeit/Animations/Anim_Attack.Anim_Attack" true :!label _label)
  (Utilities|FlowControl|Sequence
    (:then_0
      (Rendering|Components|Light|SetIntensity (Variables|Default|GetLightBase) 0.0)
      (Utilities|FlowControl|Delay 2.0)
      (bind _easein (Timeline|BaseLight PlayFromStart)
        (:Update
          (Rendering|Components|Light|SetIntensity (Variables|Default|GetLightBase) (* _easein (Variables|Default|GetBaseLightMult))))
        (:Finished
          (Utilities|FlowControl|Delay 7.0)
          (goto _label))))
    (:then_1
      (Rendering|Components|Light|SetIntensity (Variables|Default|GetStaffLight) 0.0)
      (Utilities|FlowControl|Delay 2.0)
      (bind _stafflight (Timeline|Timeline PlayFromStart)
        (:Update
          (Rendering|Components|Light|SetIntensity (Variables|Default|GetStaffLight) (* _stafflight (Variables|Default|GetStaffLightMult))))))))

(fn ConstructionScript)